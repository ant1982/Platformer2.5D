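; BP_PlatformGM is the platformer game mode that tracks the player character and respawns it at the last checkpoint when destroyed.
; One tick after BeginPlay it finds the character, binds to its OnDestroyed and passes the reference to all BPI_Interactable actors.
; RespawnPlayer spawns and possesses a new character, rebinds OnDestroyed, then sets BP_Camera as view target and retargets it.
; Interactables are not sent the new reference on respawn.
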(event Custom|RespawnPlayer
  (params (DestroyedActor :type Actor%20Object%20Reference))
  (bind _lastcheckpoint (Variables|Default|GetLastCheckPoint))
  (Utilities|IsValid _lastcheckpoint
    (:Is%20Valid
      (bind _returnvalue (Game|SpawnActorfromClass "/Game/ThirdPerson/Blueprints/BP_ThirdPersonCharacter.BP_ThirdPersonCharacter_C" (Transformation|GetActorTransform _lastcheckpoint) "Undefined" "MultiplyWithRoot" 0 0))
      (bind _output_get (Variables|Default|SetCharacterRef _returnvalue))
      (Game|BindEventtoOnDestroyed _output_get (EventDispatchers|CreateEvent :!event Custom|RespawnPlayer))
      (Pawn|Possess (Game|GetPlayerController 0) _returnvalue)
      (bind _outactors (Actor|GetAllActorsOfClass "/Game/Blueprints/BP_Camera.BP_Camera_C"))
      (Game|Player|SetViewTargetwithBlend (Game|GetPlayerController 0) (Utilities|Array|Get(acopy) _outactors) 0.0 "VTBlend_Linear" 0.0 false)
      (Variables|/Game/Blueprints/BP_Camera.BP_Camera_C|SetTargetCharacter (Utilities|Array|Get(acopy) _outactors) (Variables|Default|GetCharacterRef)))))

(event EventBeginPlay
  (Utilities|FlowControl|Sequence
    (:then_0
      (Utilities|FlowControl|DelayUntilNextTick)
      (bind _outactors (Actor|GetAllActorsOfClass "/Game/ThirdPerson/Blueprints/BP_ThirdPersonCharacter.BP_ThirdPersonCharacter_C"))
      (Utilities|IsValid (Utilities|Array|Get(acopy) _outactors)
        (:Is%20Valid
          (bind _output_get (Variables|Default|SetCharacterRef (Utilities|Array|Get(acopy) _outactors)))
          (Game|BindEventtoOnDestroyed _output_get (EventDispatchers|CreateEvent :!event Custom|RespawnPlayer))
          (bind _outactors_2 (Actor|GetAllActorswithInterface "/Game/TWE14001771/Interfaces/BPI_Interactable.BPI_Interactable_C"))
          (for _array_element _outactors_2
            (Class|BPIInteractable|SetPlayerReference(Message) _array_element (Variables|Default|GetCharacterRef))))))))

(event EventTick
  (params (DeltaSeconds :type Float%20%28single-precision%29)))

(fn ConstructionScript)