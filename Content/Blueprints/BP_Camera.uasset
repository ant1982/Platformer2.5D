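; Side-following camera actor that moves each tick toward a target character's X and Z, based on its own current Y, plus an offset.
; VInterpTo smooths the movement, with speed selected by the NormalMovement flag.
; Events set or clear the offset and arm distance; the move event also sets direction and that flag.
; Spring arm length interpolation exists only as unexecuted nodes, so distance and direction have no effect here.
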(event Custom|MoveCameraArmToNewPosition
  (params (DistanceToMove :type Float%20%28double-precision%29) (DirectionToMove :type E_CameraMoveDirection%20Enum :default "NewEnumerator0") (OffsetValue :type Vector) (Reset :type Boolean))
  (Variables|Default|SetDistance%20to%20Move DistanceToMove)
  (Variables|Default|SetOffset%20Value OffsetValue)
  (Variables|Default|SetNormalMovement Reset)
  (Variables|Default|SetDirection%20to%20Move DirectionToMove))

(event Custom|ResetCameraToOriginalPosition
  (Variables|Default|SetDistance%20to%20Move 0.0)
  (Variables|Default|SetOffset%20Value "0, 0, 0"))

(event Custom|UpdateCameraPosition
  (bind _returnvalue (Transformation|GetActorLocation))
  (bind _targetcharacter (Variables|Default|GetTargetCharacter))
  (bind _returnvalue_2 (Transformation|GetActorLocation _targetcharacter))
  (bind (_x _y _z) (Math|Vector|BreakVector _returnvalue_2))
  (Utilities|IsValid _targetcharacter
    (:Is%20Valid
      (Transformation|SetActorLocation (Math|Interpolation|VInterpTo _returnvalue (+ (Math|Vector|MakeVector _x (.Y (Math|Vector|BreakVector _returnvalue)) _z) (Variables|Default|GetOffset%20Value)) (Utilities|Time|GetWorldDeltaSeconds) (Math|Float|SelectFloat (Variables|Default|GetB) (Variables|Default|GetA) (Variables|Default|GetNormalMovement))) false false))))

(event EventBeginPlay
  (Variables|Default|SetTargetArmLength (Variables|/Script/Engine.SpringArmComponent|GetTargetArmLength (Variables|Default|GetSpringArm))))

(event EventTick
  (params (DeltaSeconds :type Float%20%28single-precision%29))
  (CallFunction|UpdateCameraPosition))

(fn ConstructionScript)