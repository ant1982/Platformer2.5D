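; A trigger volume that adjusts the game camera while the third-person character is inside it.
; On BeginPlay it caches the first BP_Camera found in the level.
; Box overlap by the character tells that camera to move its arm by the volume's DistanceToMove, with a fixed direction and offset.
; Leaving the box resets the camera to its original position.
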(event OnComponentBeginOverlap(Box)
  (params (OverlappedComponent :type Primitive%20Component%20Object%20Reference) (OtherActor :type Actor%20Object%20Reference) (OtherComp :type Primitive%20Component%20Object%20Reference) (OtherBodyIndex :type Integer) (bFromSweep :type Boolean) (SweepResult :type Hit%20Result%20Structure%20%28by%20ref%29))
  (bind _bp_camera (Variables|Default|GetBP_Camera))
  (Utilities|Casting|CastToBP_ThirdPersonCharacter OtherActor)
  (Utilities|IsValid _bp_camera
    (:Is%20Valid
      (Default|MoveCameraArmtoNewPosition _bp_camera (Variables|Default|GetDistance%20to%20Move) "NewEnumerator3" "750.000000,0.000000,0.000000" false))))

(event OnComponentEndOverlap(Box)
  (params (OverlappedComponent :type Primitive%20Component%20Object%20Reference) (OtherActor :type Actor%20Object%20Reference) (OtherComp :type Primitive%20Component%20Object%20Reference) (OtherBodyIndex :type Integer))
  (bind _bp_camera (Variables|Default|GetBP_Camera))
  (Utilities|Casting|CastToBP_ThirdPersonCharacter OtherActor)
  (Utilities|IsValid _bp_camera
    (:Is%20Valid
      (Default|ResetCameratoOriginalPosition _bp_camera))))

(event EventBeginPlay
  (bind _outactors (Actor|GetAllActorsOfClass "/Game/Blueprints/BP_Camera.BP_Camera_C"))
  (Utilities|IsValid (Utilities|Array|Get(acopy) _outactors)
    (:Is%20Valid
      (Variables|Default|SetBP_Camera (Utilities|Array|Get(acopy) _outactors)))))

(fn ConstructionScript)