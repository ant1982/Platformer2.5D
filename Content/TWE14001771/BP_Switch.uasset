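; BP_Switch is a switch that activates an array of target actors when the third-person character steps into its sphere trigger.
; On overlap, a DoOnce gate sends ActivateTargetMessage to every target and plays a Timeline that offsets the switch mesh from its starting location.
; Leaving the sphere reverses the Timeline from its end.
; The Timeline's Finished output resets the gate so the switch can fire again.
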(event OnComponentBeginOverlap(Sphere)
  (params (OverlappedComponent :type Primitive%20Component%20Object%20Reference) (OtherActor :type Actor%20Object%20Reference) (OtherComp :type Primitive%20Component%20Object%20Reference) (OtherBodyIndex :type Integer) (bFromSweep :type Boolean) (SweepResult :type Hit%20Result%20Structure%20%28by%20ref%29))
  (Utilities|Casting|CastToBP_ThirdPersonCharacter OtherActor)
  (Utilities|FlowControl|DoOnce false
    (:Completed
      (CallFunction|ActivateSwitchTargets)
      (bind _newtrack_0 (Timeline|Timeline PlayFromStart)
        (:Update
          (Transformation|SetWorldLocation (Variables|Default|GetSwitch) (+ (Variables|Default|GetStart%20Relative%20Location) _newtrack_0) false false))
        (:Finished
          (CallFunction|Reset))))))

(event OnComponentEndOverlap(Sphere)
  (params (OverlappedComponent :type Primitive%20Component%20Object%20Reference) (OtherActor :type Actor%20Object%20Reference) (OtherComp :type Primitive%20Component%20Object%20Reference) (OtherBodyIndex :type Integer))
  (Utilities|Casting|CastToBP_ThirdPersonCharacter OtherActor)
  (bind _newtrack_0 (Timeline|Timeline ReverseFromEnd)
    (:Update
      (Transformation|SetWorldLocation (Variables|Default|GetSwitch) (+ (Variables|Default|GetStart%20Relative%20Location) _newtrack_0) false false))
    (:Finished
      (CallFunction|Reset))))

(event Custom|Reset
  (Utilities|FlowControl|DoOnce false) ; enters at Reset
)

(event EventBeginPlay
  (Variables|Default|SetStart%20Relative%20Location (Transformation|GetWorldLocation (Variables|Default|GetSwitch))))

(fn ConstructionScript)

(fn ActivateSwitchTargets
  (for _array_element (Variables|Default|GetTargetActor)
    (Class|BPIUsable|ActivateTarget(Message) _array_element))
  (return))