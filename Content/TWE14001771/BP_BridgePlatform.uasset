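; Bridge platform that rotates between a start and target rotation when activated, if rotation is enabled.
; ActivateTarget waits a delay, then a DoOnce-gated timeline lerps the scene component's relative rotation and sets a return timer on completion.
; The return, also triggered by DeactivateTarget, reverses the timeline from its end at ReturnRate, then restores play rate and re-arms the gate.
; The construction script applies the start rotation.
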(event Custom|ReturnToOriginalPosition
  (Components|Timeline|SetPlayRate (Variables|Default|GetRotTimeline) (Variables|Default|GetReturnRate))
  (bind (_direction _newtrack_0) (Timeline|RotTimeline ReverseFromEnd)
    (:Update
      (Transformation|SetRelativeRotation (Variables|Default|GetScene1) (Math|Rotator|Lerp(Rotator) (Variables|Default|GetStartRotation) (Variables|Default|GetTargetRotation) _newtrack_0 (Variables|Default|GetShortest%20Path)) false false))
    (:Finished
      (switch Utilities|FlowControl|Switch|SwitchonETimelineDirection _direction
        (:Forward
          (Utilities|Time|SetTimerbyEvent (EventDispatchers|CreateEvent :!event Custom|ReturnToOriginalPosition) (Variables|Default|GetReturnDelay)))
        (:Backward
          (Components|Timeline|SetPlayRate (Variables|Default|GetRotTimeline) 1.0)
          (CallFunction|ResetTimeline))))))

(event Custom|ResetTimeline
  (Utilities|FlowControl|DoOnce false) ; enters at Reset
)

(event EventActivateTarget
  (if (Variables|Default|GetRotateIntoPosition)
    (Utilities|FlowControl|Delay (Variables|Default|GetActivationDelay))
    (Utilities|FlowControl|DoOnce false
      (:Completed
        (bind (_direction _newtrack_0) (Timeline|RotTimeline PlayFromStart)
          (:Update
            (Transformation|SetRelativeRotation (Variables|Default|GetScene1) (Math|Rotator|Lerp(Rotator) (Variables|Default|GetStartRotation) (Variables|Default|GetTargetRotation) _newtrack_0 (Variables|Default|GetShortest%20Path)) false false))
          (:Finished
            (switch Utilities|FlowControl|Switch|SwitchonETimelineDirection _direction
              (:Forward
                (Utilities|Time|SetTimerbyEvent (EventDispatchers|CreateEvent :!event Custom|ReturnToOriginalPosition) (Variables|Default|GetReturnDelay)))
              (:Backward
                (Components|Timeline|SetPlayRate (Variables|Default|GetRotTimeline) 1.0)
                (CallFunction|ResetTimeline)))))))))

(event EventDeactivateTarget
  (if (Variables|Default|GetRotateIntoPosition)
    (Components|Timeline|SetPlayRate (Variables|Default|GetRotTimeline) (Variables|Default|GetReturnRate))
    (bind (_direction _newtrack_0) (Timeline|RotTimeline ReverseFromEnd)
      (:Update
        (Transformation|SetRelativeRotation (Variables|Default|GetScene1) (Math|Rotator|Lerp(Rotator) (Variables|Default|GetStartRotation) (Variables|Default|GetTargetRotation) _newtrack_0 (Variables|Default|GetShortest%20Path)) false false))
      (:Finished
        (switch Utilities|FlowControl|Switch|SwitchonETimelineDirection _direction
          (:Forward
            (Utilities|Time|SetTimerbyEvent (EventDispatchers|CreateEvent :!event Custom|ReturnToOriginalPosition) (Variables|Default|GetReturnDelay)))
          (:Backward
            (Components|Timeline|SetPlayRate (Variables|Default|GetRotTimeline) 1.0)
            (CallFunction|ResetTimeline)))))))

(fn ConstructionScript
  (Transformation|SetRelativeRotation (Variables|Default|GetScene1) (Variables|Default|GetStartRotation) false false))