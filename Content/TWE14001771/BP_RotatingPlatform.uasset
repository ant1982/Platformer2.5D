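; Platform actor that tilts between left-side-up and right-side-up states, swapping between blue and orange plastic materials as each flip starts.
; ActivatePlatform, when enabled, plays or reverses a timeline that drives actor pitch, with a DoOnce gate blocking retriggers until the flip finishes.
; BeginPlay stores the starting rotation and sets timeline time and material for platforms not starting left-side-up.
; SetPlayerReference stores the player and binds to its OnUpdateLevel dispatcher.
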(event Custom|ActivatePlatform
  (if (Variables|Default|GetEnabled)
    (Utilities|FlowControl|DoOnce false
      (:Completed
        (CallFunction|ActivateTimeline)))))

(event Custom|ResetJump
  (Utilities|FlowControl|DoOnce false) ; enters at Reset
)

(event Custom|ActivateTimeline
  (bind _startrotation (Variables|Default|GetStartRotation))
  (bind (_roll _pitch _yaw) (Math|Rotator|BreakRotator _startrotation))
  (if (Variables|Default|GetLeftSideUp?)
    (Rendering|Material|SetMaterial (Variables|Default|GetStaticMesh) 0 "/Game/Platformer/Materials/M_Plastic_blue_Inst.M_Plastic_blue_Inst")
    (bind (_direction _newtrack_0) (Timeline|RotatingTimeline Play)
      (:Update
        (Transformation|SetActorRotation (Math|Rotator|MakeRotator _roll _newtrack_0 _yaw)))
      (:Finished
        (switch Utilities|FlowControl|Switch|SwitchonETimelineDirection _direction
          (:Forward
            (Variables|Default|SetLeftSideUp? false)
            (CallFunction|ResetJump))
          (:Backward
            (Variables|Default|SetLeftSideUp? true)
            (CallFunction|ResetJump)))))
    (else
      (Rendering|Material|SetMaterial (Variables|Default|GetStaticMesh) 0 "/Game/Platformer/Materials/M_Plastic_Orange_Inst.M_Plastic_Orange_Inst")
      (Timeline|RotatingTimeline ReverseFromEnd))))

(event EventBeginPlay
  (|CallParentFunction)
  (Variables|Default|SetStartRotation (Transformation|GetActorRotation))
  (if (not (Variables|Default|GetLeftSideUp?))
    (Components|Timeline|SetNewTime (Variables|Default|GetRotatingTimeline) 1.0)
    (Rendering|Material|SetMaterial (Variables|Default|GetStaticMesh) 0 "/Game/Platformer/Materials/M_Plastic_blue_Inst.M_Plastic_blue_Inst")))

(event Collision|EventActorBeginOverlap
  (params (OtherActor :type Actor%20Object%20Reference))
  (|CallParentFunction OtherActor) ; This node is disabled and will not be called.\nDrag off pins to build functionality.
)

(event EventTick
  (params (DeltaSeconds :type Float%20%28single-precision%29))
  (|CallParentFunction DeltaSeconds) ; This node is disabled and will not be called.\nDrag off pins to build functionality.
)

(event EventSetPlayerReference
  (params (PlayerRef :type BP%20Third%20Person%20Character%20Object%20Reference))
  (bind _output_get (Variables|Default|SetPlayer%20Ref PlayerRef))
  (EventDispatchers|BindEventtoOnUpdateLevel _output_get (EventDispatchers|CreateEvent :!event Custom|ActivatePlatform)))

(fn ConstructionScript
  (|CallParentFunction))