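; Falling platform test actor, triggered when BP_ThirdPersonCharacter overlaps its Box.
; BeginPlay caches the actor's location as StartLocation.
; After a FallDuration delay, the mesh gets physics enabled, velocity zeroed, physics disabled and its world location set to StartLocation.
; These steps run back to back with no wait for a fall; two Teleport nodes are left unconnected.
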(event OnComponentBeginOverlap(Box)
  (params (OverlappedComponent :type Primitive%20Component%20Object%20Reference) (OtherActor :type Actor%20Object%20Reference) (OtherComp :type Primitive%20Component%20Object%20Reference) (OtherBodyIndex :type Integer) (bFromSweep :type Boolean) (SweepResult :type Hit%20Result%20Structure%20%28by%20ref%29))
  (bind _staticmesh (Variables|Default|GetStaticMesh))
  (bind _staticmesh_2 (Variables|Default|GetStaticMesh))
  (Utilities|Casting|CastToBP_ThirdPersonCharacter OtherActor)
  (Utilities|FlowControl|Delay (Variables|Default|GetFall%20Duration))
  (Physics|SetSimulatePhysics _staticmesh_2 true)
  (Class|PrimitiveComponent|SetAllPhysicsLinearVelocity _staticmesh_2 "0, 0, 0" false)
  (Physics|SetSimulatePhysics _staticmesh false)
  (Transformation|SetWorldLocation _staticmesh (Variables|Default|GetStartLocation) false false))

(event EventBeginPlay
  (Variables|Default|SetStartLocation (Transformation|GetActorLocation)))

(event Collision|EventActorBeginOverlap
  (params (OtherActor :type Actor%20Object%20Reference)))

(event EventTick
  (params (DeltaSeconds :type Float%20%28single-precision%29)))

(fn ConstructionScript)